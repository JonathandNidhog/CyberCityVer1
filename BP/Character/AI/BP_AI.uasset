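; Enemy AI character with a modular samurai body that fights the player and spawns a BP_AI_Witch in its place on death.
; Damage lowers clamped health, shows the HUD health bar and alerts the AI controller to the attacker; zero health notifies the controller, then destroys the actor.
; Tick turns the health widget toward the camera and feeds the controller FarAttack.
; The right capsule damages BP_WarGirl on overlap.
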(event `self.ReceiveBeginPlay`
  ;[1 1 1] 自动走
)

(event `self.ReceiveAnyDamage`
  (params (Damage :type "Float (single-precision)") (DamageType :type "DamageType Object Reference") (InstigatedBy :type "Controller Object Reference") (DamageCauser :type "Actor Object Reference"))
  (bind _asbp_aicontroller (cast `/Game/BP/Character/AI/BP_AIController` (`AIBlueprintHelperLibrary.GetAIController` self) :!pure true))
  ;[1 1 1] 血条
  (set `self.Current HP` (`KismetMathLibrary.FClamp` (- (`self.Current HP`) Damage) 0.0 (`self.MAX HP`)))
  (`/Game/BP/ui/UI_AIHP.AIHPVisible` (`/Game/BP/ui/UI_MainUI02.UI_AIHP` (`/Game/BP/BaseGameMode/BP_HUD.MainUI02` (cast `/Game/BP/BaseGameMode/BP_HUD` (`PlayerController.GetHUD` (`GameplayStatics.GetPlayerController` 0)) :!pure true))) self)
  (`/Game/BP/Character/AI/BP_AIController.Detected` _asbp_aicontroller DamageCauser)
  (if (<= (`self.Current HP`) 0.0)
    (`/Engine/EditorBlueprintResources/StandardMacros.DoOnce` false
      (:`Completed`
        (`/Game/BP/Character/AI/BP_AIController.AIDeath` _asbp_aicontroller)
        (`PrimitiveComponent.SetCollisionEnabled` (`self.CapsuleComponent`) "NoCollision")
        (`KismetSystemLibrary.Delay` 0.2)
        (`AIBlueprintHelperLibrary.SpawnAIFromClass` "/Game/BP/Character/AI/BP_AI_Witch.BP_AI_Witch_C" null (`self.K2_GetActorLocation`) (struct) false null)
        (`self.K2_DestroyActor`)))))

(event `self.ReceiveTick`
  (params (DeltaSeconds :type "Float (single-precision)"))
  (bind _widget (`self.Widget`))
  ;[1 1 1] 血条位置
  (`SceneComponent.K2_SetWorldRotation` _widget (`KismetMathLibrary.FindLookAtRotation` (`SceneComponent.K2_GetComponentLocation` _widget) (`self.K2_GetActorLocation` (`GameplayStatics.GetPlayerCameraManager` 0))) false false)
  (`/Game/BP/Character/AI/BP_AIController.Far` (cast `/Game/BP/Character/AI/BP_AIController` (`AIBlueprintHelperLibrary.GetAIController` self) :!pure true) (`self.FarAttack`)))

(event `self.RightCapsule.OnComponentBeginOverlap`
  (params (OverlappedComponent :type "PrimitiveComponent Object Reference") (OtherActor :type "Actor Object Reference") (OtherComp :type "PrimitiveComponent Object Reference") (OtherBodyIndex :type Integer) (bFromSweep :type Boolean) (SweepResult :type "HitResult Structure (by ref)"))
  (bind _asbp_war_girl (cast `/Game/BP/Character/BP_WarGirl` OtherActor))
  (`GameplayStatics.ApplyDamage` _asbp_war_girl 5.0))

(fn `UserConstructionScript`
  (`SkinnedMeshComponent.SetLeaderPoseComponent` (`self.SK_CyberpunkSamurai_Bag`) (`self.Mesh`) true)
  (`SkinnedMeshComponent.SetLeaderPoseComponent` (`self.SK_CyberpunkSamurai_Jacket`) (`self.Mesh`) true)
  (`SkinnedMeshComponent.SetLeaderPoseComponent` (`self.SK_CyberpunkSamurai_Helmet`) (`self.Mesh`) true)
  (`SkinnedMeshComponent.SetLeaderPoseComponent` (`self.SK_CyberpunkSamurai_Hair`) (`self.Mesh`) true))